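; BP_GameState is a game state Blueprint that responds to wave state changes and handles the game over presentation.
; WaveStateChanged prints each new state on screen and acts further only on GameOver.
; On game over, an authority switch shows a separate server or client game over widget.
; It then shows the mouse cursor and sets the first player controller to UI-only input.
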(event EventWaveStateChanged
  (params (NewState :type EWaveState%20Enum :default "WaitingToStart") (OldState :type EWaveState%20Enum :default "WaitingToStart"))
  (bind _returnvalue (Game|GetPlayerController 0))
  (Development|PrintString (Utilities|String|EnumtoString NewState) true true "(R=1.000000,G=0.843627,B=0.000000,A=1.000000)" 5.0)
  (if (Utilities|Enum|Equal(Enum) NewState "GameOver")
    ;[1 1 1] On Game Over - Show Game Over Screen
    (Networking|SwitchHasAuthority
      (:Authority
        (bind _returnvalue_2 (UserInterface|CreateWidget "/Game/UI/WBP_GameOverScreenServer.WBP_GameOverScreenServer_C"))
        (UserInterface|Viewport|AddtoViewport _returnvalue_2 0))
      (:Remote
        (bind _returnvalue_3 (UserInterface|CreateWidget "/Game/UI/WBP_GameOverScreenClient.WBP_GameOverScreenClient_C"))
        (UserInterface|Viewport|AddtoViewport _returnvalue_3 0)))
    (Variables|/Script/Engine.PlayerController|SetbShowMouseCursor _returnvalue true)
    (Input|SetInputModeUIOnly _returnvalue 0 "DoNotLock")))

(fn ConstructionScript)