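; Cluster grenade actor that explodes half a second after BeginPlay, releasing smaller grenade projectiles.
; Explode plays a scaled-up explosion emitter, calls SpawnGrenade in a loop, applies radial damage and destroys the actor.
; Each SpawnGrenade call creates a half-scale, near-zero-speed BP_GrenadeProjectile and quarters the cluster's own ExplosionRadius, so the final damage radius is drastically reduced.
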(event Custom|Explode
  (bind _returnvalue (Transformation|GetActorLocation))
  (Effects|SpawnEmitteratLocation "/Game/WeaponEffects/Explosion/P_Explosion.P_Explosion" _returnvalue "0, 0, 0" "2.000000,2.000000,2.000000")
  (for _index (range 0 5)
    (CallFunction|SpawnGrenade))
  (Game|Damage|ApplyRadialDamage 1e+02 _returnvalue (Variables|Default|GetExplosionRadius) 0 0 self (Game|GetInstigatorController) false "ECC_Visibility")
  (Actor|DestroyActor))

(event Custom|SpawnGrenade
  (bind _returnvalue (Transformation|GetActorTransform))
  (bind (_location _rotation _scale) (Math|Transform|BreakTransform _returnvalue))
  (bind _returnvalue_2 (Game|SpawnActorfromClass "/Game/Blueprints/BP_GrenadeProjectile.BP_GrenadeProjectile_C" (Math|Transform|MakeTransform _location _rotation (* _scale 0.5)) "AlwaysSpawn" 0 0))
  (bind _output_get (Variables|/Script/Engine.ProjectileMovementComponent|SetInitialSpeed (Variables|/Game/Blueprints/BP_GrenadeProjectile.BP_GrenadeProjectile_C|GetProjectileMovement _returnvalue_2) 0.1))
  (Variables|/Script/Engine.ProjectileMovementComponent|SetMaxSpeed (Variables|/Game/Blueprints/BP_GrenadeProjectile.BP_GrenadeProjectile_C|GetProjectileMovement _returnvalue_2) _output_get)
  (Variables|Default|SetExplosionRadius (* (Variables|Default|GetExplosionRadius) 0.25)))

(event EventBeginPlay
  (Utilities|FlowControl|Delay 0.5)
  (CallFunction|Explode))

(fn ConstructionScript)